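; Health pickup that homes in on a ThirdPersonCharacter below max HP, then destroys itself and heals a random amount.
; Entering AttractionSphere plays a timeline that moves and scales the mesh toward the player.
; A looping-style Bobbing timeline starts on BeginPlay only from characters already overlapping AttractionSphere, and StopBobSphere halts it for injured players.
; The construction script randomizes the pickup's scale.
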(event OnComponentBeginOverlap(StopBobSphere)
  (params (OverlappedComponent :type Primitive%20Component%20Object%20Reference) (OtherActor :type Actor%20Object%20Reference) (OtherComp :type Primitive%20Component%20Object%20Reference) (OtherBodyIndex :type Integer) (bFromSweep :type Boolean) (SweepResult :type Hit%20Result%20Structure%20%28by%20ref%29))
  ;[1 1 1] Bobbing
  (bind _asthird_person_character (Utilities|Casting|CastToThirdPersonCharacter OtherActor))
  (Variables|Default|SetPlayerChar _asthird_person_character)
  (if (< (Variables|/Game/ThirdPersonBP/Blueprints/ThirdPersonCharacter.ThirdPersonCharacter_C|GetHP (Variables|Default|GetPlayerChar)) (Variables|/Game/ThirdPersonBP/Blueprints/ThirdPersonCharacter.ThirdPersonCharacter_C|GetMaxHP (Variables|Default|GetPlayerChar)))
    (bind _bobbing (Timeline|Bobbing Stop)
      (:Update
        (Transformation|SetRelativeLocation (Variables|Default|GetHP_Pickup) (Math|Vector|Lerp(Vector) (stale EventBeginPlay _output_get) "0,0.000000,80.000000" _bobbing) false false)))))

(event OnComponentBeginOverlap(AttractionSphere)
  (params (OverlappedComponent :type Primitive%20Component%20Object%20Reference) (OtherActor :type Actor%20Object%20Reference) (OtherComp :type Primitive%20Component%20Object%20Reference) (OtherBodyIndex :type Integer) (bFromSweep :type Boolean) (SweepResult :type Hit%20Result%20Structure%20%28by%20ref%29))
  (bind _hp_pickup (Variables|Default|GetHP_Pickup))
  (bind _hp_pickup_2 (Variables|Default|GetHP_Pickup))
  (bind _returnvalue (Transformation|GetWorldScale _hp_pickup_2))
  ;[1 1 1] Collection and Healing
  (bind _asthird_person_character (Utilities|Casting|CastToThirdPersonCharacter OtherActor))
  (Utilities|IsValid _asthird_person_character
    (:Is%20Valid
      (Variables|Default|SetPlayerChar _asthird_person_character)
      (if (< (Variables|/Game/ThirdPersonBP/Blueprints/ThirdPersonCharacter.ThirdPersonCharacter_C|GetHP (Variables|Default|GetPlayerChar)) (Variables|/Game/ThirdPersonBP/Blueprints/ThirdPersonCharacter.ThirdPersonCharacter_C|GetMaxHP (Variables|Default|GetPlayerChar)))
        (bind (_direction _distance _size) (Timeline|Attraction Play)
          (:Update
            (Transformation|SetWorldScale3D (Variables|Default|GetHP_Pickup) (Math|Vector|MakeVector (* (.x _returnvalue) _size) (* (.y _returnvalue) _size) (* (.z _returnvalue) _size)))
            (Utilities|IsValid (Variables|Default|GetPlayerChar)
              (:Is%20Valid
                (Utilities|IsValid _hp_pickup
                  (:Is%20Valid
                    (Transformation|SetWorldLocation _hp_pickup (Math|Vector|Lerp(Vector) (Transformation|GetWorldLocation (Variables|Default|GetHP_Pickup)) (Transformation|GetActorLocation (Variables|Default|GetPlayerChar)) _distance) false false))))))
          (:Finished
            (Actor|DestroyActor)
            (Default|Heal (Variables|Default|GetPlayerChar) (Math|Random|RandomFloatinRange 3e+02 75.0))))))))

(event EventBeginPlay
  ;[1 1 1] Bobbing
  (for _array_element (Collision|GetOverlappingActors (Variables|Default|GetAttractionSphere) "/Script/Engine.Actor" :!class /Script/Engine.PrimitiveComponent)
    (bind _asthird_person_character (Utilities|Casting|CastToThirdPersonCharacter _array_element))
    (Variables|Default|SetPlayerChar _asthird_person_character)
    (bind _output_get (Variables|Default|SetBase%20Location "0, 0,30.000000"))
    (bind _bobbing (Timeline|Bobbing Play)
      (:Update
        (Transformation|SetRelativeLocation (Variables|Default|GetHP_Pickup) (Math|Vector|Lerp(Vector) _output_get "0,0.000000,80.000000" _bobbing) false false)))))

(fn ConstructionScript
  (bind _hp_pickup (Variables|Default|GetHP_Pickup))
  (bind _returnvalue (Transformation|GetWorldScale _hp_pickup))
  (Variables|Default|SetSizeSeed (Math|Random|RandomFloatinRange 0.2 0.7))
  (Transformation|SetWorldScale3D _hp_pickup (Math|Vector|MakeVector (* (Variables|Default|GetSizeSeed) (.x _returnvalue)) (* (Variables|Default|GetSizeSeed) (.y _returnvalue)) (* (Variables|Default|GetSizeSeed) (.z _returnvalue)))))