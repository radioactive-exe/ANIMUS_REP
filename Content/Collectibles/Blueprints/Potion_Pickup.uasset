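; Health potion pickup that adds one to the player character's potion count when collected.
; On BeginPlay it caches the player's ThirdPersonCharacter and plays a timeline that bobs the mesh vertically by lerping its relative location.
; When a ThirdPersonCharacter overlaps the collection capsule, it increments the cached player's HealthPotionCount, destroys itself and plays a bottle-clinking sound at its location.
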(event OnComponentBeginOverlap(CollectionCapsule)
  (params (OverlappedComponent :type Primitive%20Component%20Object%20Reference) (OtherActor :type Actor%20Object%20Reference) (OtherComp :type Primitive%20Component%20Object%20Reference) (OtherBodyIndex :type Integer) (bFromSweep :type Boolean) (SweepResult :type Hit%20Result%20Structure%20%28by%20ref%29))
  (bind _playerchar (Variables|Default|GetPlayerChar))
  (Utilities|Casting|CastToThirdPersonCharacter OtherActor)
  (Variables|/Game/ThirdPersonBP/Blueprints/ThirdPersonCharacter.ThirdPersonCharacter_C|SetHealthPotionCount _playerchar (+ (Variables|/Game/ThirdPersonBP/Blueprints/ThirdPersonCharacter.ThirdPersonCharacter_C|GetHealthPotionCount _playerchar) 1.0))
  (Actor|DestroyActor)
  (Audio|PlaySoundatLocation "/Game/SFX/SoundFX/416288__fugeni__empty-beer-bottles-clinking-clanking.416288__fugeni__empty-beer-bottles-clinking-clanking" (Transformation|GetActorLocation) "0, 0, 0" 1.0 1.0 0.0 0 0 0))

(event EventBeginPlay
  (bind _asthird_person_character (Utilities|Casting|CastToThirdPersonCharacter (Game|GetPlayerCharacter 0)))
  (Variables|Default|SetPlayerChar _asthird_person_character)
  (Variables|Default|SetBase%20Location "0, 0,80.000000")
  (bind _bobbing (Timeline|Timeline_0 Play)
    (:Update
      (Transformation|SetRelativeLocation (Variables|Default|GetStaticMesh1) (Math|Vector|Lerp(Vector) "0, 0,50.000000" "0,0.000000,90.000000" _bobbing) false false))))

(event Collision|EventActorBeginOverlap
  (params (OtherActor :type Actor%20Object%20Reference)))

(event EventTick
  (params (DeltaSeconds :type Float%20%28single-precision%29)))

(fn ConstructionScript)