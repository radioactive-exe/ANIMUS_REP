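; Checkpoint flag that records the player's respawn transform and saves progress on first overlap with its sphere.
; Overlap adds the flag to Save1's used list before the character cast, then saves through the game mode, glows yellow, plays a ding and shows a widget.
; The respawn point comes from a downward trace at SpawnCone, with yaw fed by the flag's Z location.
; On BeginPlay, used flags lose their sphere and glow yellow.
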(event OnComponentBeginOverlap(Sphere)
  (params (OverlappedComponent :type Primitive%20Component%20Object%20Reference) (OtherActor :type Actor%20Object%20Reference) (OtherComp :type Primitive%20Component%20Object%20Reference) (OtherBodyIndex :type Integer) (bFromSweep :type Boolean) (SweepResult :type Hit%20Result%20Structure%20%28by%20ref%29))
  (bind _returnvalue (SaveGame|LoadGamefromSlot "Save1"))
  (bind _asbp_save_game (Utilities|Casting|CastToBP_SaveGame _returnvalue))
  (if (not (Utilities|Array|ContainsItem (Variables|/Game/ThirdPersonBP/Blueprints/BP_SaveGame.BP_SaveGame_C|GetCheckpointUsed _asbp_save_game) self))
    (Utilities|Array|Add (Variables|/Game/ThirdPersonBP/Blueprints/BP_SaveGame.BP_SaveGame_C|GetCheckpointUsed _asbp_save_game) self)
    (SaveGame|SaveGametoSlot _asbp_save_game "Save1")
    (bind _asthird_person_game_mode (Utilities|Casting|CastToThirdPersonGameMode (Game|GetGameMode)))
    (bind _asthird_person_character (Utilities|Casting|CastToThirdPersonCharacter OtherActor))
    (bind _returnvalue_2 (|GetCPSpawnPos _asthird_person_character)
      (:Out
        (Variables|/Game/ThirdPersonBP/Blueprints/ThirdPersonCharacter.ThirdPersonCharacter_C|SetLastCPTransform _asthird_person_character _returnvalue_2)
        (Default|SaveGame _asthird_person_game_mode)
        (Components|DestroyComponent (Variables|Default|GetSphere))
        (Utilities|Casting|CastToThirdPersonCharacter OtherActor)
        (Rendering|Material|SetMaterial (Variables|Default|GetFlag) 0 "/Game/Animus_Demo/Islands_And_Meshes_Main/Materials/Yellow_Glow.Yellow_Glow")
        (Audio|PlaySoundatLocation "/Game/SFX/SoundFX/267337__gkillhour__ding-4.267337__gkillhour__ding-4" (Transformation|GetWorldLocation (Variables|Default|GetStaticMesh)) "0, 0, 0" 1.0 1.0 0.0 0 0 0)
        (bind _returnvalue_3 (UserInterface|CreateWidget "/Game/UI/Widgets/Checkpoint_Widget.Checkpoint_Widget_C"))
        (UserInterface|Viewport|AddtoViewport _returnvalue_3 0)))))

(event EventBeginPlay
  (bind _returnvalue (SaveGame|LoadGamefromSlot "Save1"))
  (bind _asbp_save_game (Utilities|Casting|CastToBP_SaveGame _returnvalue))
  (if (Utilities|Array|ContainsItem (Variables|/Game/ThirdPersonBP/Blueprints/BP_SaveGame.BP_SaveGame_C|GetCheckpointUsed _asbp_save_game) self)
    (Components|DestroyComponent (Variables|Default|GetSphere))
    (Rendering|Material|SetMaterial (Variables|Default|GetFlag) 0 "/Game/Animus_Demo/Islands_And_Meshes_Main/Materials/Yellow_Glow.Yellow_Glow")))

(fn ConstructionScript)