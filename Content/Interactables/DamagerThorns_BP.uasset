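; DamagerThorns_BP is an interactable thorns hazard that repeatedly damages the ThirdPersonCharacter while it overlaps the DamageBox.
; Entering the box stores the cast character and starts a fast looping timer on the ConstantDamage event.
; Each tick of that timer calls the character's Damage with a random amount, provided the stored reference is valid.
; When a ThirdPersonCharacter leaves the box, the stored timer handle is cleared and invalidated.
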(event OnComponentBeginOverlap(DamageBox)
  (params (OverlappedComponent :type Primitive%20Component%20Object%20Reference) (OtherActor :type Actor%20Object%20Reference) (OtherComp :type Primitive%20Component%20Object%20Reference) (OtherBodyIndex :type Integer) (bFromSweep :type Boolean) (SweepResult :type Hit%20Result%20Structure%20%28by%20ref%29))
  (bind _asthird_person_character (Utilities|Casting|CastToThirdPersonCharacter OtherActor))
  (bind _returnvalue (Utilities|Time|SetTimerbyEvent (delegate Custom|ConstantDamage) 0.1 true))
  (Variables|Default|SetTimeHandler _returnvalue))

(event OnComponentEndOverlap(DamageBox)
  (params (OverlappedComponent :type Primitive%20Component%20Object%20Reference) (OtherActor :type Actor%20Object%20Reference) (OtherComp :type Primitive%20Component%20Object%20Reference) (OtherBodyIndex :type Integer))
  (Utilities|Casting|CastToThirdPersonCharacter OtherActor)
  (Utilities|Time|ClearandInvalidateTimerbyHandle (Variables|Default|GetTimeHandler)))

(event Custom|ConstantDamage
  (Utilities|IsValid (stale OnComponentBeginOverlap(DamageBox) _asthird_person_character)
    (:Is%20Valid
      (Default|Damage (stale OnComponentBeginOverlap(DamageBox) _asthird_person_character) (Math|Random|RandomFloatinRange 1e+02 1.5e+02)))))

(event EventBeginPlay)

(event Collision|EventActorBeginOverlap
  (params (OtherActor :type Actor%20Object%20Reference)))

(event EventTick
  (params (DeltaSeconds :type Float%20%28single-precision%29)))

(fn ConstructionScript)