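; Battle gate actor that opens with a short camera cutscene once its associated enemy quest spawner reports all clear.
; BeginPlay takes the first MEGA_Enemy_Quest_BP_Child in the level, and Tick polls its AllClear flag behind a DoOnce.
; It blends the view to CutsceneCam, plays a sound and swings both gate halves open via a timeline, then blends back to the player's follow camera.
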(event EventBeginPlay
  (bind _outactors (Actor|GetAllActorsOfClass "/Game/Quest_System/MEGA_Enemy_Quest_BP_Child.MEGA_Enemy_Quest_BP_Child_C"))
  (Variables|Default|SetAssociatedSpawner (Utilities|Array|Get(acopy) _outactors)))

(event Collision|EventActorBeginOverlap
  (params (OtherActor :type Actor%20Object%20Reference)))

(event EventTick
  (params (DeltaSeconds :type Float%20%28single-precision%29))
  (if (Variables|/Game/Quest_System/Enemy_Quest_BP.Enemy_Quest_BP_C|GetAllClear (Variables|Default|GetAssociatedSpawner))
    (Utilities|FlowControl|DoOnce false
      (:Completed
        (Game|Player|SetViewTargetwithBlend (Game|GetPlayerController 0) (Components|GetOwner (Variables|Default|GetCutsceneCam)) 2.0 "VTBlend_EaseInOut" 3.0 false)
        (Utilities|FlowControl|Delay 1.0)
        (Audio|PlaySoundatLocation "/Game/SFX/HugeGate_Open.HugeGate_Open" (Transformation|GetActorLocation) "0, 0, 0" 1.0 1.0 0.0 0 0 0)
        (bind _open (Timeline|GateOpen Play)
          (:Update
            (Transformation|SetRelativeRotation (Variables|Default|GetGate_L) (Math|Rotator|MakeRotator 0.0 0.0 (* _open -9e+01)) false false)
            (Transformation|SetRelativeRotation (Variables|Default|GetGate_R) (Math|Rotator|MakeRotator 0.0 0.0 (+ (* _open 9e+01) 1.8e+02)) false false))
          (:Finished
            (Utilities|FlowControl|Delay 1.0)
            (Game|Player|SetViewTargetwithBlend (Game|GetPlayerController 0) (Components|GetOwner (Variables|/Game/ThirdPersonBP/Blueprints/ThirdPersonCharacter.ThirdPersonCharacter_C|GetFollowCamera (.AsThird%20Person%20Character (Utilities|Casting|CastToThirdPersonCharacter (Game|GetPlayerCharacter 0))))) 1.3 "VTBlend_EaseInOut" 3.0 false)))))))

(fn ConstructionScript)