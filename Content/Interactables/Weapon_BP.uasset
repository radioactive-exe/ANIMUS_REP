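; Pickup melee weapon that the player equips to a pelvis socket and uses to damage enemies.
; PickUpWeapon drops any equipped weapon at this one's position, or shows a sword-controls tooltip if none is held, then attaches itself to the character mesh.
; Mesh overlaps with an enemy capsule while the player is attacking trigger aggro, deal heavy fixed damage and flag the enemy as seeing the player.
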(event OnComponentBeginOverlap(StaticMesh)
  (params (OverlappedComponent :type Primitive%20Component%20Object%20Reference) (OtherActor :type Actor%20Object%20Reference) (OtherComp :type Primitive%20Component%20Object%20Reference) (OtherBodyIndex :type Integer) (bFromSweep :type Boolean) (SweepResult :type Hit%20Result%20Structure%20%28by%20ref%29))
  (bind _asenemy_blueprint (Utilities|Casting|CastToEnemy_Blueprint OtherActor))
  (Utilities|IsValid _asenemy_blueprint
    (:Is%20Valid
      (Utilities|Casting|CastToCapsuleComponent OtherComp)
      (if (Variables|/Game/ThirdPersonBP/Blueprints/ThirdPersonCharacter.ThirdPersonCharacter_C|GetAttacking (Variables|Default|GetPlayerCharRef))
        (Default|Aggro _asenemy_blueprint)
        (Default|Damage _asenemy_blueprint 1e+03)
        (Utilities|IsValid _asenemy_blueprint
          (:Is%20Valid
            (if (not (Variables|/Game/ThirdPersonBP/Blueprints/Enemy_Blueprint.Enemy_Blueprint_C|GetCanSeePlayer _asenemy_blueprint))
              (Variables|/Game/ThirdPersonBP/Blueprints/Enemy_Blueprint.Enemy_Blueprint_C|SetCanSeePlayer _asenemy_blueprint true))))))))

(event EventBeginPlay
  (bind _asthird_person_character (Utilities|Casting|CastToThirdPersonCharacter (Game|GetPlayerCharacter 0)))
  (Utilities|IsValid _asthird_person_character
    (:Is%20Valid
      (Variables|Default|SetPlayerCharRef _asthird_person_character))))

(event EventPickUpWeapon
  (bind _returnvalue (Game|GetPlayerCharacter 0))
  (bind _defaultsceneroot (Variables|Default|GetDefaultSceneRoot))
  (bind _asthird_person_character (Utilities|Casting|CastToThirdPersonCharacter _returnvalue))
  (Utilities|IsValid (Variables|/Game/ThirdPersonBP/Blueprints/ThirdPersonCharacter.ThirdPersonCharacter_C|GetEquippedWeapon (.AsThird%20Person%20Character (Utilities|Casting|CastToThirdPersonCharacter (Game|GetPlayerCharacter 0))))
    (:Is%20Valid
      (Transformation|DetachFromActor (Variables|/Game/ThirdPersonBP/Blueprints/ThirdPersonCharacter.ThirdPersonCharacter_C|GetEquippedWeapon (.AsThird%20Person%20Character (Utilities|Casting|CastToThirdPersonCharacter (Game|GetPlayerCharacter 0)))) "KeepRelative" "KeepRelative" "KeepRelative")
      (Transformation|SetActorLocationAndRotation (Variables|/Game/ThirdPersonBP/Blueprints/ThirdPersonCharacter.ThirdPersonCharacter_C|GetEquippedWeapon (.AsThird%20Person%20Character (Utilities|Casting|CastToThirdPersonCharacter (Game|GetPlayerCharacter 0)))) (Transformation|GetWorldLocation _defaultsceneroot) (Transformation|GetWorldRotation _defaultsceneroot)))
    (:Is%20Not%20Valid
      (bind _returnvalue_2 (UserInterface|CreateWidget "/Game/UI/Widgets/ToolTip.ToolTip_C"))
      (Rendering|Components|TextRender|SetText (Variables|/Game/UI/Widgets/ToolTip.ToolTip_C|GetTipText _returnvalue_2) "[HINT: Press LMB to draw your sword, or to attack if it's already drawn, and press RMB to sheathe your sword.]")
      (UserInterface|Viewport|AddtoViewport _returnvalue_2 0)))
  (Variables|/Game/ThirdPersonBP/Blueprints/ThirdPersonCharacter.ThirdPersonCharacter_C|SetEquippedWeapon _asthird_person_character self)
  (Transformation|AttachComponentToComponent (Variables|/Script/Engine.Character|GetMesh _asthird_person_character) "Weapon_Pelvis" "SnapToTarget" "SnapToTarget" "KeepRelative" true))

(fn ConstructionScript)