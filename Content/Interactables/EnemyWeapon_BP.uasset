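; Enemy weapon actor that damages the player character when its mesh hits them during an attack.
; On static mesh overlap, it requires the character's capsule component and a valid, living EnemyRef that is attacking, then calls Damage on the character with a fixed amount.
; Disconnected pickup logic for swapping the player's equipped weapon and socketing it at the pelvis remains in the graph but never runs.
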(event OnComponentBeginOverlap(StaticMesh)
  (params (OverlappedComponent :type Primitive%20Component%20Object%20Reference) (OtherActor :type Actor%20Object%20Reference) (OtherComp :type Primitive%20Component%20Object%20Reference) (OtherBodyIndex :type Integer) (bFromSweep :type Boolean) (SweepResult :type Hit%20Result%20Structure%20%28by%20ref%29))
  (bind _enemyref (Variables|Default|GetEnemyRef))
  (bind _asthird_person_character (Utilities|Casting|CastToThirdPersonCharacter OtherActor))
  (Utilities|IsValid _asthird_person_character
    (:Is%20Valid
      (Utilities|Casting|CastToCapsuleComponent OtherComp)
      (Utilities|IsValid _enemyref
        (:Is%20Valid
          (if (Variables|/Game/ThirdPersonBP/Blueprints/Enemy_Blueprint.Enemy_Blueprint_C|GetAttacking _enemyref)
            (if (Variables|/Game/ThirdPersonBP/Blueprints/Enemy_Blueprint.Enemy_Blueprint_C|GetisAlive _enemyref)
              (Default|Damage _asthird_person_character 1e+02))))))))

(fn ConstructionScript)