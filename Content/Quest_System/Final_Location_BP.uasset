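; Quest destination actor that completes a player's quest when they stand inside its box.
; Each Tick it takes the first overlapping ThirdPersonCharacter and searches their active quests for one referencing this actor.
; On a match, a DoOnce completes that quest on the character, then finds NPC_Blueprint actors with the same quest name.
; Each matching NPC gets its completion event, followed by the character's TrickQuestion call and this actor's destruction.
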(event EventTick
  (params (DeltaSeconds :type Float%20%28single-precision%29))
  (bind _asthird_person_character (Utilities|Casting|CastToThirdPersonCharacter (Utilities|Array|Get(acopy) (Collision|GetOverlappingActors (Variables|Default|GetBox) "/Game/ThirdPersonBP/Blueprints/ThirdPersonCharacter.ThirdPersonCharacter_C" :!class /Script/Engine.PrimitiveComponent))))
  (for _array_element (Variables|/Game/ThirdPersonBP/Blueprints/ThirdPersonCharacter.ThirdPersonCharacter_C|GetActiveQuests _asthird_person_character)
    (if (== self (.actorreference (Variables|/Game/Quest_System/BP_Quest.BP_Quest_C|GetQuestInfo _array_element)))
      (Utilities|FlowControl|DoOnce false
        (:Completed
          (Default|QuestComplete _asthird_person_character _array_element)
          (bind _outactors (Actor|GetAllActorsOfClass "/Game/ThirdPersonBP/Blueprints/NPC_Blueprint.NPC_Blueprint_C"))
          (for _array_element_2 _outactors
            (if (Utilities|Enum|Equal(Enum) (.questname (Variables|/Game/Quest_System/BP_Quest.BP_Quest_C|GetQuestInfo _array_element)) (.questname (Variables|/Game/ThirdPersonBP/Blueprints/NPC_Blueprint.NPC_Blueprint_C|GetQuestRef _array_element_2)))
              (Default|EventQuestComplete _array_element_2)
              (Default|TrickQuestion _asthird_person_character)
              (Actor|DestroyActor))))))))

(fn ConstructionScript)