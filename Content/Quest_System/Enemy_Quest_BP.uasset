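; Quest encounter spawner that creates a small random group of enemies on BeginPlay and completes its linked quest once none remain.
; Enemies spawn at random reachable nearby points with random yaw, register this actor as ParentSpawner, and are counted as living.
; Tick watches for a zero count, then once clears player combat, completes quests referencing this actor, notifies matching NPCs with a sound, and destroys itself.
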(event Custom|SpawnEnemies
  (params (NumOfEnemies :type Integer) (SpawnDistance :type Float%20%28single-precision%29))
  (for _index (range 0 (- NumOfEnemies 1))
    (bind _returnvalue (Game|SpawnActorfromClass "/Game/ThirdPersonBP/Blueprints/Enemy_Blueprint.Enemy_Blueprint_C" (Math|Transform|MakeTransform (.RandomLocation (AI|Navigation|GetRandomReachablePointinRadius (Transformation|GetActorLocation) SpawnDistance 0 0)) (Math|Rotator|MakeRotator 0.0 0.0 (Math|Random|RandomFloatinRange 0.0 3.6e+02))) "AdjustIfPossibleButDontSpawnIfColliding" 0 0))
    (Utilities|IsValid _returnvalue
      (:Is%20Valid
        (Utilities|Array|Add (Variables|Default|GetEnemies) _returnvalue)
        (Variables|/Game/ThirdPersonBP/Blueprints/Enemy_Blueprint.Enemy_Blueprint_C|SetParentSpawner _returnvalue self))))
  (for _array_element (Variables|Default|GetEnemies)
    (Utilities|IsValid _array_element
      (:Is%20Valid
        (if (== (Variables|/Game/ThirdPersonBP/Blueprints/Enemy_Blueprint.Enemy_Blueprint_C|GetParentSpawner _array_element) self)
          (Math|Integer|IncrementInt (Variables|Default|GetNumOfLivingEnemies))
          (else
            (Actor|DestroyActor _array_element)))))))

(event EventBeginPlay
  (CallFunction|SpawnEnemies (Math|Random|RandomIntegerinRange 2 5) 4e+02))

(event EventTick
  (params (DeltaSeconds :type Float%20%28single-precision%29))
  (if (== (Variables|Default|GetNumOfLivingEnemies) 0)
    (Utilities|FlowControl|DoOnce false
      (:Completed
        (Variables|Default|SetAllClear true)
        (bind _asthird_person_character (Utilities|Casting|CastToThirdPersonCharacter (Game|GetPlayerCharacter 0)))
        (Variables|/Game/ThirdPersonBP/Blueprints/ThirdPersonCharacter.ThirdPersonCharacter_C|SetIsInCombat _asthird_person_character false)
        (for _array_element (Variables|/Game/ThirdPersonBP/Blueprints/ThirdPersonCharacter.ThirdPersonCharacter_C|GetActiveQuests _asthird_person_character)
          (if (== self (.actorreference (Variables|/Game/Quest_System/BP_Quest.BP_Quest_C|GetQuestInfo _array_element)))
            (Default|QuestComplete _asthird_person_character _array_element)
            (bind _outactors (Actor|GetAllActorsOfClass "/Game/ThirdPersonBP/Blueprints/NPC_Blueprint.NPC_Blueprint_C"))
            (for _array_element_2 _outactors
              (if (Utilities|Enum|Equal(Enum) (.questname (Variables|/Game/Quest_System/BP_Quest.BP_Quest_C|GetQuestInfo _array_element)) (.questname (Variables|/Game/ThirdPersonBP/Blueprints/NPC_Blueprint.NPC_Blueprint_C|GetQuestRef _array_element_2)))
                (Audio|PlaySound2D "/Game/SFX/QuestComplete.QuestComplete" 1.0 1.0 0.0 0 0)
                (Default|EventQuestComplete _array_element_2)
                (Actor|DestroyActor)))))))))

(fn ConstructionScript)