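; Quest location trigger that completes the player's matching active quest when their character overlaps its box.
; It finds the quest whose actor reference is this actor, completes it once, then notifies NPCs with the same quest name.
; On an NPC match, it plays a sound, swaps the first interactible crystal found for a happy crystal, calls Damage on the player and sets their max HP.
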(event OnComponentBeginOverlap(Box)
  (params (OverlappedComponent :type Primitive%20Component%20Object%20Reference) (OtherActor :type Actor%20Object%20Reference) (OtherComp :type Primitive%20Component%20Object%20Reference) (OtherBodyIndex :type Integer) (bFromSweep :type Boolean) (SweepResult :type Hit%20Result%20Structure%20%28by%20ref%29))
  (bind _asthird_person_character (Utilities|Casting|CastToThirdPersonCharacter OtherActor))
  (Utilities|IsValid _asthird_person_character
    (:Is%20Valid
      (for _array_element (Variables|/Game/ThirdPersonBP/Blueprints/ThirdPersonCharacter.ThirdPersonCharacter_C|GetActiveQuests _asthird_person_character)
        (Utilities|IsValid _array_element
          (:Is%20Valid
            (if (== self (.actorreference (Variables|/Game/Quest_System/BP_Quest.BP_Quest_C|GetQuestInfo _array_element)))
              (Utilities|FlowControl|DoOnce false
                (:Completed
                  (Default|QuestComplete _asthird_person_character _array_element)
                  (bind _outactors (Actor|GetAllActorsOfClass "/Game/ThirdPersonBP/Blueprints/NPC_Blueprint.NPC_Blueprint_C"))
                  (for _array_element_2 _outactors
                    (Utilities|IsValid _array_element_2
                      (:Is%20Valid
                        (if (Utilities|Enum|Equal(Enum) (.questname (Variables|/Game/Quest_System/BP_Quest.BP_Quest_C|GetQuestInfo _array_element)) (.questname (Variables|/Game/ThirdPersonBP/Blueprints/NPC_Blueprint.NPC_Blueprint_C|GetQuestRef _array_element_2)))
                          (Audio|PlaySound2D "/Game/SFX/QuestComplete.QuestComplete" 1.0 1.0 0.0 0 0)
                          (Default|EventQuestComplete _array_element_2)
                          (bind _outactors_2 (Actor|GetAllActorsOfClass "/Game/ThirdPersonBP/Blueprints/InteractibleCrystal_Blueprint.InteractibleCrystal_Blueprint_C"))
                          (Variables|Default|SetCrystalSpawnTransform (Transformation|GetActorTransform (Utilities|Array|Get(acopy) _outactors_2)))
                          (Actor|DestroyActor (Utilities|Array|Get(acopy) _outactors_2))
                          (Game|SpawnActorfromClass "/Game/ThirdPersonBP/Blueprints/HappyCrystal_BP.HappyCrystal_BP_C" (Variables|Default|GetCrystalSpawnTransform) "Undefined" 0 0)
                          (bind _asthird_person_character_2 (Utilities|Casting|CastToThirdPersonCharacter (Game|GetPlayerCharacter 0)))
                          (Utilities|IsValid _asthird_person_character_2
                            (:Is%20Valid
                              (Default|Damage _asthird_person_character_2 2.5e+02)
                              (Variables|/Game/ThirdPersonBP/Blueprints/ThirdPersonCharacter.ThirdPersonCharacter_C|SetMaxHP _asthird_person_character_2 7.5e+02))))))))))))))))

(fn ConstructionScript)