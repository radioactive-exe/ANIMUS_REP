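; Final battle quest parent actor that runs successive enemy waves by spawning enemy quest child actors at its own transform.
; BeginPlay spawns the first wave spawner, then Tick polls its AllClear flag and spawns a replacement, incrementing WaveIndex until the wave limit.
; Once the last spawner is clear, a DoOnce sets AllDone and disables the actor's tick.
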(event EventBeginPlay
  (bind _returnvalue (Game|SpawnActorfromClass "/Game/Quest_System/FinalBattleEnemyQuest_BP_Child.FinalBattleEnemyQuest_BP_Child_C" (Transformation|GetActorTransform) "Undefined" 0 0))
  (Variables|Default|SetSpawner _returnvalue))

(event EventTick
  (params (DeltaSeconds :type Float%20%28single-precision%29))
  (if (< (Variables|Default|GetWaveIndex) 3)
    (if (Variables|/Game/Quest_System/Enemy_Quest_BP.Enemy_Quest_BP_C|GetAllClear (Variables|Default|GetSpawner))
      (bind _returnvalue (Game|SpawnActorfromClass "/Game/Quest_System/FinalBattleEnemyQuest_BP_Child.FinalBattleEnemyQuest_BP_Child_C" (Transformation|GetActorTransform) "Undefined" 0 0))
      (Variables|Default|SetSpawner _returnvalue)
      (Math|Integer|IncrementInt (Variables|Default|GetWaveIndex)))
    (elif (Variables|/Game/Quest_System/Enemy_Quest_BP.Enemy_Quest_BP_C|GetAllClear (Variables|Default|GetSpawner))
      (Utilities|FlowControl|DoOnce false
        (:Completed
          (Variables|Default|SetAllDone true)
          (Actor|Tick|SetActorTickEnabled false))))))

(fn ConstructionScript)