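; Location_BP is a trigger actor that completes a location quest when the player reaches it.
; When a ThirdPersonCharacter overlaps its Box, it searches that character's ActiveQuests for one whose ActorReference is this actor.
; A DoOnce gate then completes the quest on the character and finds every NPC_Blueprint with a matching quest name, playing the completion sound and calling EventQuestComplete on each.
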(event OnComponentBeginOverlap(Box)
  (params (OverlappedComponent :type Primitive%20Component%20Object%20Reference) (OtherActor :type Actor%20Object%20Reference) (OtherComp :type Primitive%20Component%20Object%20Reference) (OtherBodyIndex :type Integer) (bFromSweep :type Boolean) (SweepResult :type Hit%20Result%20Structure%20%28by%20ref%29))
  (bind _asthird_person_character (Utilities|Casting|CastToThirdPersonCharacter OtherActor))
  (for _array_element (Variables|/Game/ThirdPersonBP/Blueprints/ThirdPersonCharacter.ThirdPersonCharacter_C|GetActiveQuests _asthird_person_character)
    (if (== self (.actorreference (Variables|/Game/Quest_System/BP_Quest.BP_Quest_C|GetQuestInfo _array_element)))
      (Utilities|FlowControl|DoOnce false
        (:Completed
          (Default|QuestComplete _asthird_person_character _array_element)
          (bind _outactors (Actor|GetAllActorsOfClass "/Game/ThirdPersonBP/Blueprints/NPC_Blueprint.NPC_Blueprint_C"))
          (for _array_element_2 _outactors
            (if (Utilities|Enum|Equal(Enum) (.questname (Variables|/Game/Quest_System/BP_Quest.BP_Quest_C|GetQuestInfo _array_element)) (.questname (Variables|/Game/ThirdPersonBP/Blueprints/NPC_Blueprint.NPC_Blueprint_C|GetQuestRef _array_element_2)))
              (Audio|PlaySound2D "/Game/SFX/QuestComplete.QuestComplete" 1.0 1.0 0.0 0 0)
              (Default|EventQuestComplete _array_element_2))))))))

(fn ConstructionScript)